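; Physics-driven ball actor that travels at a constant speed along diagonal directions in the horizontal plane.
; BeginPlay launches it diagonally with a velocity-change impulse.
; Every Tick clamps velocity to BallSpeed and snaps heading to the nearest diagonal by rotating 45 degrees, rounding yaw to 90-degree steps and rotating back.
; The snapped direction also prints each frame as debug output.
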(event `self.ReceiveTick`
  (params (DeltaSeconds :type "Float (single-precision)"))
  (`self.VelocityAndAngle`))

(event `self.ReceiveBeginPlay`
  (`self.LaunchBall`))

(event `LaunchBall`
  (`PrimitiveComponent.AddImpulse` (`self.Ball`) (10.0 -10.0 0.0) "None" true))

(event `VelocityAndAngle`
  (bind _returnvalue (`KismetMathLibrary.MakeRotator` 0.0 0.0 45.0))
  (bind _ballspeed (`self.BallSpeed`))
  (bind _returnvalue_2 (`PrimitiveComponent.GetPhysicsLinearVelocity` (`self.Ball`) "None"))
  (bind _returnvalue_3 (`KismetMathLibrary.ClampVectorSize` _returnvalue_2 _ballspeed _ballspeed))
  (bind (_returnvalue_roll _returnvalue_pitch _returnvalue_yaw) (`KismetMathLibrary.BreakRotator` (`KismetMathLibrary.MakeRotFromX` (`KismetMathLibrary.GreaterGreater_VectorRotator` _returnvalue_3 _returnvalue))))
  (bind _returnvalue_4 (`KismetMathLibrary.LessLess_VectorRotator` (`KismetMathLibrary.Conv_RotatorToVector` (`KismetMathLibrary.MakeRotator` 0.0 0.0 (* (`KismetMathLibrary.Round` (/ _returnvalue_yaw 90.0)) 90.0))) _returnvalue))
  (`PrimitiveComponent.SetPhysicsLinearVelocity` (`self.Ball`) (* _returnvalue_4 (`KismetMathLibrary.VSize` _returnvalue_3)) false "None")
  (`KismetSystemLibrary.PrintString` (`KismetStringLibrary.Conv_VectorToString` _returnvalue_4)))

(fn `UserConstructionScript`)